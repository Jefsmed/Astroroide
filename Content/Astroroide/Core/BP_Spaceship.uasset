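; Networked player spaceship Character for the Astroroide game, with flying movement relative to control yaw, health, death and sound feedback.
; A multicast event applies the selected ship's mesh, color material and stats, while another creates the HUD with all spaceships and starts music.
; Held fire repeats at the ship's bullet rate through a server event, which spawns up to four bullets, then recycles them round-robin as a pool.
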(event Custom|ConfigureSpaceshipByPlayerID
  (params (Material :type Material%20Interface%20Object%20Reference) (SpaceshipSelected :type S%20Player%20Space%20Ships%20Structure))
  (bind (_mesh _bulletrate _acceleration _healthpoints _initialdamage) (Utilities|Struct|BreakSPlayerSpaceShips SpaceshipSelected))
  ;[0.01179 0.08912 1] Configure spaceship - Network multicast
  (bind _output_get (Variables|Default|SetMyColorPlayer Material))
  (Rendering|Material|SetMaterial (Variables|Character|GetMesh) 1 _output_get)
  (Components|SkeletalMesh|SetSkeletalMeshAsset (Variables|Character|GetMesh) _mesh)
  (Variables|Default|SetBulletRate _bulletrate)
  (bind _output_get_2 (Variables|Default|SetAcceleration _acceleration))
  (Variables|/Script/Engine.CharacterMovementComponent|SetMaxFlySpeed (Variables|Character|GetCharacterMovement) _output_get_2)
  (Variables|Default|SetHealth _healthpoints)
  (Variables|Default|SetInitialDamage _initialdamage))

(event Custom|CreateHUD
  ;[1 1 1] Create Game HUD - Network Multicast and owning Client
  (bind _outactors (Actor|GetAllActorsOfClass (Utilities|GetClass self)))
  (bind _output_get (Variables|Default|SetAllSpaceships _outactors))
  (for _array_element _output_get
    (CallFunction|Create)))

(event Custom|Create
  ;[1 1 1] Create Game HUD - Network Multicast and owning Client
  (Utilities|FlowControl|DoOnce false
    (:Completed
      (bind _returnvalue (UserInterface|CreateWidget "/Game/Astroroide/UI/WBP_GameHud.WBP_GameHud_C" 0 (Variables|Default|GetAllSpaceships)))
      (UserInterface|Viewport|AddtoViewport _returnvalue 0)
      (Audio|PlaySound2D "/Game/Retro_8Bit_Sounds/Music/Cues/music_bytes_the_retro_adventure_Cue.music_bytes_the_retro_adventure_Cue" 0.4 1.0 0.0 0 0))))

(event EventTick
  (params (DeltaSeconds :type Float%20%28single-precision%29))
  (bind _returnvalue (Transformation|GetActorLocation))
  (Transformation|SetActorLocation (Math|Vector|MakeVector (.x _returnvalue) (.y _returnvalue) 0.0) false false))

(event Game|Damage|EventAnyDamage
  (params (Damage :type Float%20%28single-precision%29) (DamageType :type Damage%20Type%20Object%20Reference) (InstigatedBy :type Controller%20Object%20Reference) (DamageCauser :type Actor%20Object%20Reference))
  (bind _output_get (Variables|Default|SetHealth (- (Variables|Default|GetHealth) (Math|Float|Truncate Damage))))
  (if (== _output_get 0)
    (Audio|PlaySound2D "/Game/Retro_8Bit_Sounds/Explosion/Cues/retro_explosion_deep_01_Cue.retro_explosion_deep_01_Cue" 1.0 1.0 0.0 0 0)
    (Actor|DestroyActor)
    (else
      (Audio|PlaySound2D "/Game/Retro_8Bit_Sounds/Impacts/Cues/retro_impact_colorful_02_Cue.retro_impact_colorful_02_Cue" 1.0 1.0 0.0 0 0))))

(event Custom|NormalShot
  (bind _self self)
  ;[1 1 1] Input event responsible for firing the spaceship's normal shot - Roda somente nos clientes
  (if (<= (Utilities|Array|Length (Variables|Default|GetBulletsFired)) 3)
    (bind _returnvalue (Game|SpawnActorfromClass "/Game/Astroroide/Core/BP_Bullet.BP_Bullet_C" (Transformation|GetWorldTransform (Variables|Default|GetSpawnBullet)) "Undefined" _self _self))
    (Default|MovifyVelocity _returnvalue (Math|Vector|GetForwardVector (Transformation|GetActorRotation)))
    (Utilities|Array|Add (Variables|Default|GetBulletsFired) _returnvalue)
    (else
      (Transformation|SetActorTransform (Utilities|Array|Get(acopy) (Variables|Default|GetBulletsFired) (Variables|Default|GetBulletsFiredAgain)) (Transformation|GetWorldTransform (Variables|Default|GetSpawnBullet)) true true)
      (Default|MovifyVelocity (Utilities|Array|Get(acopy) (Variables|Default|GetBulletsFired) (Variables|Default|GetBulletsFiredAgain)) (Math|Vector|GetForwardVector (Transformation|GetActorRotation)))
      (Actor|SetOwner (Utilities|Array|Get(acopy) (Variables|Default|GetBulletsFired) (Variables|Default|GetBulletsFiredAgain)) self)
      (bind _result (Math|Integer|IncrementInt (Variables|Default|GetBulletsFiredAgain))
        (:%20%20
          (if (== _result 4)
            (Variables|Default|SetBulletsFiredAgain 0)))))))

(event EventIMoveForward/Backward
  (params (AxisValue :type Float%20%28double-precision%29))
  ;[1 1 1] Basic Movement
  (Pawn|Input|AddMovementInput (Math|Vector|GetForwardVector (Math|Rotator|MakeRotator 0.0 0.0 (.yaw (Pawn|GetControlRotation :!class /Script/Engine.Pawn)))) AxisValue false))

(event EventIMoveRight/Left
  (params (AxisValue :type Float%20%28double-precision%29))
  ;[1 1 1] Basic Movement
  (Pawn|Input|AddMovementInput (Math|Vector|GetRightVector (Math|Rotator|MakeRotator 0.0 0.0 (.yaw (Pawn|GetControlRotation :!class /Script/Engine.Pawn)))) AxisValue false))

(event EventINormalShot
  (params (Pressed :type Boolean))
  ;[1 1 1] Input event responsible for firing the spaceship's normal shot - Roda somente nos clientes
  (if Pressed
    (if (Variables|Default|GetFirstNormalShot) :!label _label
      (Variables|Default|SetFirstNormalShot false)
      (CallFunction|NormalShot :!label _label_2)
      (Audio|PlaySound2D "/Game/Retro_8Bit_Sounds/Weapons/Cues/retro_laser_gun_shoot_37_Cue.retro_laser_gun_shoot_37_Cue" 1.0 1.0 0.0 0 0)
      (goto _label)
      (else
        (Utilities|FlowControl|Delay (Variables|Default|GetBulletRate))
        (Utilities|FlowControl|Sequence
          (:then_0
            (if Pressed
              (goto _label_2)
              (else
                (goto _label_3 Reset))))
          (:then_1
            _)))))
  (Utilities|FlowControl|DoOnce true :!label _label_3
    (:Completed
      (Variables|Default|SetFirstNormalShot true))))

(fn ConstructionScript)