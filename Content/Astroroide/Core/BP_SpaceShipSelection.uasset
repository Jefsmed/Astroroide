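; Hangar actor for choosing the player spaceship, storing the selection on the Astroroide player controller and defaulting to Fighter when none is set.
; The selected ship's mesh and data come from DT_PlayerSpaceships and feed the skeletal mesh and selection widget.
; Two timelines move the mesh along a spline: one flies the current ship out, then the other brings the next one in.
; Widget buttons are disabled during these animations.
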(event Custom|NextSpaceship
  (params (Spaceship%20Selected :type FEPlayerSpaceships%20Enum :default "None"))
  ;[1 1 1] Select Next Spaceship
  (Class|AstroroideController|SetSpaceshipSelected (Variables|Default|GetAs%20PlayerController) Spaceship%20Selected)
  (CallFunction|StartfortheNextSpaceship))

(event Custom|EnterSelectSpaceship
  ;[1 1 1] Enter the Hangar for select spaceship
  (if (Utilities|Enum|Equal(Enum) (Class|AstroroideController|GetSpaceshipSelected (Variables|Default|GetAs%20PlayerController)) "None")
    (Class|AstroroideController|SetSpaceshipSelected (Variables|Default|GetAs%20PlayerController) "Fighter"))
  (CallFunction|ShowNextSpaceship))

(event Custom|ShowNextSpaceship
  (bind _spline (Variables|Default|GetSpline))
  ;[1 1 1] Animation - show the next spaceship
  (bind _returnvalue (Utilities|GetDataTableRow "/Game/Astroroide/DataTable/DT_PlayerSpaceships.DT_PlayerSpaceships" (Utilities|String|StringToName (Utilities|String|EnumtoString (Variables|/Script/Astroroide.AstroroideController|GetSpaceshipSelected (Variables|Default|GetAs%20PlayerController)))))
    (:then
      (Components|SkeletalMesh|SetSkeletalMeshAsset (Variables|Default|GetSkeletalMesh) (Utilities|Struct|BreakSPlayerSpaceShips (.spaceship _returnvalue)))
      (Default|SpaceshipinHangar (Variables|Default|GetWBP_SpaceshipSelection) (.spaceship _returnvalue) (Class|AstroroideController|GetSpaceshipSelected (Variables|Default|GetAs%20PlayerController)))
      (Default|DisableButtons (Variables|Default|GetWBP_SpaceshipSelection))
      (bind _alpha (Timeline|TL_NextSpaceship PlayFromStart)
        (:Update
          (Transformation|SetRelativeLocationAndRotation (Variables|Default|GetSkeletalMesh) (.location (Spline|GetTransformatDistanceAlongSpline _spline (Math|Float|Lerp 0.0 (Spline|GetDistanceAlongSplineatSplinePoint _spline 1) _alpha) "Local" false)) (.rotation (Spline|GetTransformatDistanceAlongSpline _spline (Math|Float|Lerp 0.0 (Spline|GetDistanceAlongSplineatSplinePoint _spline 1) _alpha) "Local" false)) false false))
        (:Finished
          (Default|EnableButtons (Variables|Default|GetWBP_SpaceshipSelection)))))))

(event Custom|StartForTheNextSpaceship
  (bind _spline (Variables|Default|GetSpline))
  ;[1 1 1] Start next spaceship
  (Default|DisableButtons (Variables|Default|GetWBP_SpaceshipSelection))
  (bind _alpha (Timeline|TL_StartForNextSpaceship PlayFromStart)
    (:Update
      (Transformation|SetRelativeLocationAndRotation (Variables|Default|GetSkeletalMesh) (.location (Spline|GetTransformatDistanceAlongSpline _spline (Math|Float|Lerp (Spline|GetDistanceAlongSplineatSplinePoint _spline 1) (Spline|GetDistanceAlongSplineatSplinePoint _spline 2) _alpha) "Local" false)) (.rotation (Spline|GetTransformatDistanceAlongSpline _spline (Math|Float|Lerp (Spline|GetDistanceAlongSplineatSplinePoint _spline 1) (Spline|GetDistanceAlongSplineatSplinePoint _spline 2) _alpha) "Local" false)) false false))
    (:Finished
      (CallFunction|ShowNextSpaceship))))

(event EventBeginPlay
  (bind _asastroroide_controller (Utilities|Casting|CastToAstroroideController (Game|GetPlayerController 0)))
  (Variables|Default|SetAs%20PlayerController _asastroroide_controller))

(fn ConstructionScript)