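; BP_PowerUp is a pickup actor for the Astroroide game that takes on a random power-up look when it spawns.
; On BeginPlay it picks a random row from DT_PowerUps and applies that row's mesh and scale to its static mesh component.
; Overlap with a BP_Spaceship only prints the ship's name; no power-up effect is applied yet.
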(event OnComponentBeginOverlap(Mesh)
  (params (OverlappedComponent :type Primitive%20Component%20Object%20Reference) (OtherActor :type Actor%20Object%20Reference) (OtherComp :type Primitive%20Component%20Object%20Reference) (OtherBodyIndex :type Integer) (bFromSweep :type Boolean) (SweepResult :type Hit%20Result%20Structure%20%28by%20ref%29))
  (bind _asbp_spaceship (Utilities|Casting|CastToBP_Spaceship OtherActor))
  (Development|PrintString (Utilities|GetDisplayName _asbp_spaceship)))

(event Custom|PowerUpSpawned
  (bind _mesh (Variables|Default|GetMesh))
  (bind _outrownames (DataTable|GetDataTableRowNames "/Game/Astroroide/DataTable/DT_PowerUps.DT_PowerUps"))
  (bind _returnvalue (Utilities|GetDataTableRow "/Game/Astroroide/DataTable/DT_PowerUps.DT_PowerUps" (Utilities|Array|Get(acopy) _outrownames (Math|Random|RandomIntegerinRange 0 (- (Utilities|Array|Length _outrownames) 1))))
    (:then
      (Components|StaticMesh|SetStaticMesh _mesh (.mesh _returnvalue))
      (Transformation|SetRelativeScale3D _mesh (Math|Conversions|ToVector(Float) (.meshscale _returnvalue))))))

(event EventBeginPlay
  (CallFunction|PowerUpSpawned))

(fn ConstructionScript)