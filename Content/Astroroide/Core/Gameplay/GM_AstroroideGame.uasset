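; Game mode for an Astroroide match, running it from player registration to restart.
; BeginPlay polls controllers for ten seconds, positions spaceships at PlayerStarts, then starts play after BP_Universe's intro cinematic.
; A recursive one-second timer updates players and lerps spawners toward faster, smaller asteroids.
; Time-out shows results; in sessions, a restart countdown (decrementing by zero) precedes server travel or session end, based on only the first spaceship's vote.
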(event Custom|ConfigureSpaceships
  ;[0.8125 0.7534 0.05078] Position and register the spaceships of all players in the game.
  (for (_array_element _array_index) (Variables|Network|GetAllPlayers)
    (bind _aspc_astroroide_gameplay (Utilities|Casting|CastToPC_AstroroideGameplay _array_element))
    (Transformation|SetActorTransform (Pawn|GetControlledPawn _aspc_astroroide_gameplay) (Transformation|GetActorTransform (Utilities|Array|Get(acopy) (Variables|Network|GetAllPlayersStart) _array_index)) false true)
    (bind _asbp_spaceship (Utilities|Casting|CastToBP_Spaceship (Pawn|GetControlledPawn _aspc_astroroide_gameplay)))
    (Utilities|Array|Add (Variables|Network|GetAllSpaceships) _asbp_spaceship)))

(event Custom|GetAllPlayersInMatch
  ;[1 0.9225 0] Searches and registers in the list all the players that entered the match.
  (if (Variables|Network|GetSearchPlayers)
    (bind _outactors (Actor|GetAllActorsOfClass "/Script/Engine.PlayerController"))
    (Variables|Network|SetAllPlayers _outactors)
    (for (_array_element _array_index) (Variables|Network|GetAllPlayers)
      (bind _aspc_astroroide_gameplay (Utilities|Casting|CastToPC_AstroroideGameplay _array_element))
      (Variables|/Game/Astroroide/Core/Gameplay/PC_AstroroideGameplay.PC_AstroroideGameplay_C|SetColorID _aspc_astroroide_gameplay (Utilities|Array|Get(acopy) (Variables|Network|GetColor%20ID) _array_index)))
    (Utilities|FlowControl|Delay 0.2)
    (CallFunction|GetAllPlayersinMatch)))

(event Custom|CustomEvent_1
  ;[1 0 0 1 30] Starts the reset process. If all players agree with the restart, it will reset the game map with the current players connected. If someone doesn't agree, the session will be terminated and everyone will be sent to the main menu.
  (Widget|RemovefromParent (stale Custom|MatchTimer _returnvalue))
  (bind _returnvalue (UserInterface|CreateWidget "/Game/Astroroide/UI/WBP_LoadingGame.WBP_LoadingGame_C"))
  (UserInterface|Viewport|AddtoViewport _returnvalue 0)
  (if (Variables|Default|GetRestart%20Match)
    (Development|ExecuteConsoleCommand "servertravel L_Gameplay" (Game|GetPlayerController 0))
    (else
      (|EndSession (Game|GetPlayerController 0)
        (:OnSuccess
          (Game|OpenLevel(byObjectReference) "/Game/Maps/L_MainMenu.L_MainMenu"))))))

(event Custom|CustomEvent
  ;[0.02826 0.1927 0.0271] Preparation for matchgame.
  ;;[0.08632 0.5885 0.08276] Countdown to release player controls and start the match.
  (Utilities|FlowControl|Delay 2.0)
  (for _array_element (Variables|Network|GetAllSpaceships)
    (Default|StartMatchgame _array_element))
  (Audio|PlaySound2D "/Game/Retro_8Bit_Sounds/Music/Cues/music_8bit_jammer_Cue.music_8bit_jammer_Cue" 1.0 1.0 0.0 0 0)
  ;;[0.04125 0.2812 0.03955] Start counting the match and release the game functions.
  (CallFunction|MatchTimer)
  (for _array_element_2 (Variables|Network|GetAllPlayers)
    (bind _aspc_astroroide_gameplay (Utilities|Casting|CastToPC_AstroroideGameplay _array_element_2))
    (Default|EventGameplayReleased _aspc_astroroide_gameplay))
  (bind _outactors (Actor|GetAllActorsOfClass "/Game/Astroroide/Core/Gameplay/BP_SpawnEnemies.BP_SpawnEnemies_C"))
  (bind _output_get (Variables|Gameplay|SetSpawnEnemies _outactors))
  (for _array_element_3 _output_get
    (Default|StartSpawnEnemies _array_element_3)))

(event Custom|MatchTimer
  ;[0.04645 0.05452 0.4955] Match timer. It will also establish the difficulty arc of the game.
  (bind _output_get (Variables|MatchTimer|SetMatchTimerSecond (- (Variables|MatchTimer|GetMatchTimerSecond) 1)))
  (if (< _output_get 0)
    (Variables|MatchTimer|SetMatchTimerSecond 59)
    (bind _output_get_2 (Variables|MatchTimer|SetMatchTimerMinute (- (Variables|MatchTimer|GetMatchTimerMinute) 1)))
    (if (< _output_get_2 0)
      ;[0.4583 0.02387 0.02387] Timer reaching zero will destroy all asteroids and stop spawning anymore.
      (Variables|MatchTimer|SetMatchTimerSecond 0)
      (Variables|MatchTimer|SetMatchTimerMinute 0)
      (for _array_element (Variables|Gameplay|GetSpawnEnemies)
        (Default|EventEndMatch _array_element))
      ;[0.3854 0.3574 0.02409] Blocks the controllers, removes the game interface and puts the results of all players on the screen. Checks if players are connected in a session to activate the restart timer.
      (for _array_element_2 (Variables|Network|GetAllPlayers)
        (bind _aspc_astroroide_gameplay (Utilities|Casting|CastToPC_AstroroideGameplay _array_element_2))
        (Default|EventGameplayEndMatch _aspc_astroroide_gameplay))
      (for _array_element_3 (Variables|Network|GetAllSpaceships)
        (Default|RemoveWidgetGameplay _array_element_3)
        (Utilities|FlowControl|Delay 0.2)
        (Default|CreateWidgetEndMatch _array_element_3))
      (bind _bisinsession (Class|AdvancedSessionsLibrary|IsPlayerinSession (Class|AdvancedSessionsLibrary|GetUniqueNetIDfromPlayerState (Variables|/Script/Engine.Controller|GetPlayerState (Utilities|Array|Get(acopy) (Variables|Network|GetAllPlayers))))))
      (if _bisinsession
        ;[1 1 1] Timer for restarting the game.
        (bind _output_get_3 (Variables|Default|SetRestartTimerMatch (- (Variables|Default|GetRestartTimerMatch) 0) :!label _label))
        (if (< _output_get_3 0)
          (Variables|Default|SetRestartTimerMatch 0)
          ;[1 1 1] Checks if all players agree to the restart.
          (bind _array_element_4 (Utilities|Array|ForEachLoopwithBreak (Variables|Network|GetAllSpaceships) :!label _label_2)
            (:LoopBody
              (if (Variables|/Game/Astroroide/Core/Gameplay/BP_Spaceship.BP_Spaceship_C|GetRestartMatch _array_element_4)
                (Variables|Default|SetRestart%20Match true)
                (goto _label_2 Break)
                (else
                  (Variables|Default|SetRestart%20Match false)
                  (goto _label_2 Break))))
            (:Completed
              ;[1 0 0 1 30] Starts the reset process. If all players agree with the restart, it will reset the game map with the current players connected. If someone doesn't agree, the session will be terminated and everyone will be sent to the main menu.
              (Viewport|RemoveAllWidgets)
              (bind _returnvalue (UserInterface|CreateWidget "/Game/Astroroide/UI/WBP_Fade.WBP_Fade_C"))
              (UserInterface|Viewport|AddtoViewport _returnvalue 0)
              (Default|StartFadeOut _returnvalue)
              (EventDispatchers|BindEventtoFinishFadeOut _returnvalue (delegate Custom|CustomEvent_1))))
          (else
            (Utilities|FlowControl|Delay 1.0)
            (for _array_element_5 (Variables|Network|GetAllPlayers)
              (bind _aspc_astroroide_gameplay_2 (Utilities|Casting|CastToPC_AstroroideGameplay _array_element_5))
              (Variables|/Game/Astroroide/Core/Gameplay/PC_AstroroideGameplay.PC_AstroroideGameplay_C|SetRestartTimeMatch _aspc_astroroide_gameplay_2 (Variables|Default|GetRestartTimerMatch)))
            (goto _label))))
      (else
        (Utilities|FlowControl|Delay 1.0 :!label _label_3)
        (CallFunction|MatchTimer)
        (for _array_element_6 (Variables|Network|GetAllPlayers)
          (bind _aspc_astroroide_gameplay_3 (Utilities|Casting|CastToPC_AstroroideGameplay _array_element_6))
          (Default|UpdateMatchTimer _aspc_astroroide_gameplay_3 (Variables|MatchTimer|GetMatchTimerMinute) (Variables|MatchTimer|GetMatchTimerSecond)))
        ;[0.08632 0.5885 0.08276] The more time you spend in the game, the faster the enemies appear and the smaller their size in the game.
        (for _array_element_7 (Variables|Gameplay|GetSpawnEnemies)
          (Variables|/Game/Astroroide/Core/Gameplay/BP_SpawnEnemies.BP_SpawnEnemies_C|SetMaxSpawnTimer _array_element_7 (Math|Float|Lerp 0.0 5.0 (/ (- (* (+ (Variables|MatchTimer|GetMatchTimerMinute) 1) 60) (- 60 (Variables|MatchTimer|GetMatchTimerSecond))) 1.8e+02)))
          (Variables|/Game/Astroroide/Core/Gameplay/BP_SpawnEnemies.BP_SpawnEnemies_C|SetMaxAsteroidsScale _array_element_7 (Math|Float|Lerp 2.0 5.0 (/ (- (* (+ (Variables|MatchTimer|GetMatchTimerMinute) 1) 60) (- 60 (Variables|MatchTimer|GetMatchTimerSecond))) 1.8e+02))))))
    (else
      (goto _label_3))))

(event EventBeginPlay
  ;[0.02826 0.1927 0.0271] Preparation for matchgame.
  ;;[0.04125 0.2812 0.03955] Starts an event that will search and register all players who have logged in to the match.
  (CallFunction|GetAllPlayersinMatch)
  ;;[0.04125 0.2812 0.03955] Identifies and saves the information of all players stats on the map.
  (bind _outactors (Actor|GetAllActorsOfClass "/Script/Engine.PlayerStart"))
  (Variables|Network|SetAllPlayersStart _outactors)
  ;;[1 0.9225 0] Waiting time for players to register before starting the match.
  (Utilities|FlowControl|Delay 1e+01)
  ;;[0.08632 0.5885 0.08276] This boolean will stop the new players scan loop in the match.
  (Variables|Network|SetSearchPlayers false)
  (CallFunction|ConfigureSpaceships) ; Configures all players' spaceships\nas they choose.
  ;;[0.08632 0.5885 0.08276] Defines the game camera for all players.
  (bind _outactors_2 (Actor|GetAllActorsOfClass "/Game/Astroroide/Core/Gameplay/BP_GameplayCamera.BP_GameplayCamera_C"))
  (Default|ConfigurGameplayCamera (Utilities|Array|Get(acopy) _outactors_2))
  ;;[0.1467 1 0.1406] Creates the game screen and removes the players' loadscreen.
  (for _array_element (Variables|Network|GetAllSpaceships)
    (Default|CreateHUD _array_element))
  (for _array_element_2 (Variables|Network|GetAllPlayers)
    (bind _aspc_astroroide_gameplay (Utilities|Casting|CastToPC_AstroroideGameplay _array_element_2))
    (Default|RemoveLoadingScreen _aspc_astroroide_gameplay))
  ;;[0.08632 0.5885 0.08276] Countdown to release player controls and start the match.
  (bind _outactors_3 (Actor|GetAllActorsOfClass "/Game/Astroroide/Assets/BP_Universe.BP_Universe_C"))
  (Default|CinematicBeforeGameplay (Utilities|Array|Get(acopy) _outactors_3))
  (EventDispatchers|BindEventtoFinishAnimBGameplay (Utilities|Array|Get(acopy) _outactors_3) (delegate Custom|CustomEvent)))

(event EventPostLogin
  (params (NewPlayer :type Player%20Controller%20Object%20Reference))
  ;[0.05729 0.05729 0.05729] Registers in Game mode the first player controller that logged into the map.
  (Utilities|Array|Add (Variables|Network|GetAllPlayers) NewPlayer))

(fn ConstructionScript)