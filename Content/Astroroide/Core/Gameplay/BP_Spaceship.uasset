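; Player-controlled multiplayer spaceship for Astroroide, handling flight input, firing, damage, respawn and match widgets.
; On BeginPlay it multicasts mesh, color and stats from the selected DT_PlayerSpaceships row, then a looping timer pins Z to zero.
; Held fire repeats at BulletRate through a server event that recycles a ten-bullet pool.
; Zero health hides and disables the ship, moves it to the first PlayerStart and revives it after a delay.
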(event Custom|ConfigureSpaceshipByPlayerID
  (params (Material :type Material%20Interface%20Object%20Reference) (SpaceshipSelected :type S%20Player%20Space%20Ships%20Structure))
  (bind (_mesh _bulletrate _acceleration _healthpoints _initialdamage) (Utilities|Struct|BreakSPlayerSpaceShips SpaceshipSelected))
  ;[0.01179 0.08912 1] Configure spaceship - Network multicast
  (Rendering|Material|SetMaterialbyName (Variables|Character|GetMesh) "M_PlayerMaterial" Material)
  (Components|SkeletalMesh|SetSkeletalMeshAsset (Variables|Character|GetMesh) _mesh)
  (Variables|Default|SetBulletRate _bulletrate)
  (bind _output_get (Variables|Default|SetAcceleration _acceleration))
  (Variables|/Script/Engine.CharacterMovementComponent|SetMaxFlySpeed (Variables|Character|GetCharacterMovement) _output_get)
  (bind _output_get_2 (Variables|Default|SetHealth _healthpoints))
  (Variables|Gameplay|SetMaxHealth _output_get_2)
  (Variables|Default|SetInitialDamage _initialdamage))

(event Custom|CreateHUD
  ;[1 1 1] Create Game HUD - Network Multicast and owning Client
  (bind _outactors (Actor|GetAllActorsOfClass (Utilities|GetClass self)))
  (bind _output_get (Variables|Default|SetAllSpaceships _outactors))
  (for _array_element _output_get
    (CallFunction|CreateWidgetGameplay)))

(event Custom|CreateWidgetGameplay
  ;[1 1 1] Create Game HUD - Network Multicast and owning Client
  (bind _returnvalue (UserInterface|CreateWidget "/Game/Astroroide/UI/Gameplay/WBP_Gameplay.WBP_Gameplay_C" 0 (Variables|Default|GetAllSpaceships)))
  (bind _output_get (Variables|Widget|SetGameHUD _returnvalue))
  (UserInterface|Viewport|AddtoViewport _output_get 0))

(event Custom|ActorZeroAxisZ
  (bind _returnvalue (Transformation|GetActorLocation))
  ;[1 1 1] Simulates the tick event to keep the actor at zero z-axis value.
  (Transformation|SetActorLocation (Math|Vector|MakeVector (.x _returnvalue) (.y _returnvalue) 0.0) false false))

(event Custom|StartMatchgame
  ;[1 1 1] Create Game HUD - Network Multicast and owning Client
  (Default|StartMatchgame (Variables|Widget|GetGameHUD)))

(event Custom|RemoveWidgetGameplay
  ;[1 1 1] Create Game HUD - Network Multicast and owning Client
  (Widget|RemovefromParent (Variables|Widget|GetGameHUD)))

(event Custom|CreateWidgetEndMatch
  ;[1 1 1] Open the end of match widget
  (bind _outactors (Actor|GetAllActorsOfClass (Utilities|GetClass self)))
  (bind _output_get (Variables|Default|SetAllSpaceships _outactors))
  (for _array_element _output_get
    (CallFunction|CreateEndMatch)))

(event Custom|CreateEndMatch
  ;[1 1 1] Open the end of match widget
  (bind _returnvalue (UserInterface|CreateWidget "/Game/Astroroide/UI/Gameplay/WBP_EndMatch.WBP_EndMatch_C" 0 (Variables|Default|GetAllSpaceships) self))
  (bind _output_get (Variables|Widget|SetEndMatch _returnvalue))
  (UserInterface|Viewport|AddtoViewport _output_get 0)
  (Variables|Default|SetIsDeath true)
  (Default|AddResult _output_get))

(event EventBeginPlay
  ;[1 1 1] Begin play
  (Utilities|FlowControl|Delay 1.0)
  (bind _aspc_astroroide_gameplay (Utilities|Casting|CastToPC_AstroroideGameplay (Components|GetOwner)))
  (bind _returnvalue (Utilities|GetDataTableRow "/Game/Astroroide/DataTable/DT_PlayerSpaceships.DT_PlayerSpaceships" (Utilities|String|StringToName (Utilities|String|EnumtoString (Class|AstroroideController|GetSpaceshipSelected _aspc_astroroide_gameplay))))
    (:then
      (CallFunction|ConfigureSpaceshipbyPlayerID (Variables|/Game/Astroroide/Core/Gameplay/PC_AstroroideGameplay.PC_AstroroideGameplay_C|GetColorID _aspc_astroroide_gameplay) (.spaceship _returnvalue))
      ;[1 1 1] Simulates the tick event to keep the actor at zero z-axis value.
      (Utilities|Time|SetTimerbyEvent (delegate Custom|ActorZeroAxisZ) 0.01 true))))

(event Game|Damage|EventAnyDamage
  (params (Damage :type Float%20%28single-precision%29) (DamageType :type Damage%20Type%20Object%20Reference) (InstigatedBy :type Controller%20Object%20Reference) (DamageCauser :type Actor%20Object%20Reference))
  (bind _output_get (Variables|Default|SetHealth (- (Variables|Default|GetHealth) (Math|Float|Truncate Damage))))
  (if (== _output_get 0)
    (Audio|PlaySound2D "/Game/Retro_8Bit_Sounds/Explosion/Cues/retro_explosion_deep_01_Cue.retro_explosion_deep_01_Cue" 1.0 1.0 0.0 0 0)
    (Variables|Default|SetIsDeath true)
    (Math|Integer|IncrementInt (Variables|Gameplay|GetDeaths)
      (:%20%20
        (Rendering|SetVisibility (Variables|Character|GetMesh) false false)
        (Collision|SetCollisionEnabled (Variables|Default|GetCapsuleComponent) "NoCollision")
        (Pawn|Components|CharacterMovement|SetMovementMode (Variables|Character|GetCharacterMovement) "MOVE_None" 0)
        (bind _outactors (Actor|GetAllActorsOfClass "/Script/Engine.PlayerStart"))
        (Transformation|SetActorTransform (Transformation|GetActorTransform (Utilities|Array|Get(acopy) _outactors)) false true)
        (Utilities|FlowControl|Delay 3.0)
        (Variables|Default|SetIsDeath false)
        (Variables|Default|SetHealth (Variables|Gameplay|GetMaxHealth))
        (Rendering|SetVisibility (Variables|Character|GetMesh) true false)
        (Pawn|Components|CharacterMovement|SetMovementMode (Variables|Character|GetCharacterMovement) "MOVE_Flying" 0)
        (Collision|SetCollisionEnabled (Variables|Default|GetCapsuleComponent) "QueryAndPhysics")
        (Audio|PlaySound2D "/Game/Retro_8Bit_Sounds/Teleport/Cues/retro_teleport_warp_effect_43_Cue.retro_teleport_warp_effect_43_Cue" 1.0 1.0 0.0 0 0)))
    (else
      (Audio|PlaySound2D "/Game/Retro_8Bit_Sounds/Impacts/Cues/retro_impact_colorful_02_Cue.retro_impact_colorful_02_Cue" 1.0 1.0 0.0 0 0))))

(event Custom|NormalShot
  (bind _self self)
  ;[0.09237 0.2 0.9062] Input event responsible for firing the spaceship's normal shot
  (if (<= (Utilities|Array|Length (Variables|SpaceshipConfig|GetBulletsFired)) 9)
    (bind _returnvalue (Game|SpawnActorfromClass "/Game/Astroroide/Core/Gameplay/BP_Bullet.BP_Bullet_C" (Transformation|GetWorldTransform (Variables|Default|GetSpawnBullet)) "Undefined" _self _self))
    (Default|MovifyVelocity _returnvalue (Math|Vector|GetForwardVector (Transformation|GetActorRotation)))
    (Utilities|Array|Add (Variables|SpaceshipConfig|GetBulletsFired) _returnvalue)
    (else
      (Transformation|SetActorTransform (Utilities|Array|Get(acopy) (Variables|SpaceshipConfig|GetBulletsFired) (Variables|SpaceshipConfig|GetBulletsFiredAgain)) (Transformation|GetWorldTransform (Variables|Default|GetSpawnBullet)) true true)
      (Default|MovifyVelocity (Utilities|Array|Get(acopy) (Variables|SpaceshipConfig|GetBulletsFired) (Variables|SpaceshipConfig|GetBulletsFiredAgain)) (Math|Vector|GetForwardVector (Transformation|GetActorRotation)))
      (Actor|SetOwner (Utilities|Array|Get(acopy) (Variables|SpaceshipConfig|GetBulletsFired) (Variables|SpaceshipConfig|GetBulletsFiredAgain)) self)
      (bind _result (Math|Integer|IncrementInt (Variables|SpaceshipConfig|GetBulletsFiredAgain))
        (:%20%20
          (if (== _result 10)
            (Variables|SpaceshipConfig|SetBulletsFiredAgain 0)))))))

(event EventIMoveForward/Backward
  (params (AxisValue :type Float%20%28double-precision%29))
  ;[1 1 1] Basic Movement
  (Pawn|Input|AddMovementInput (Math|Vector|GetForwardVector (Math|Rotator|MakeRotator 0.0 0.0 (.yaw (Pawn|GetControlRotation :!class /Script/Engine.Pawn)))) AxisValue false))

(event EventIMoveRight/Left
  (params (AxisValue :type Float%20%28double-precision%29))
  ;[1 1 1] Basic Movement
  (Pawn|Input|AddMovementInput (Math|Vector|GetRightVector (Math|Rotator|MakeRotator 0.0 0.0 (.yaw (Pawn|GetControlRotation :!class /Script/Engine.Pawn)))) AxisValue false))

(event EventINormalShot
  (params (Pressed :type Boolean))
  ;[0.09237 0.2 0.9062] Input event responsible for firing the spaceship's normal shot
  (if Pressed
    (if (Variables|Gameplay|GetFirstNormalShot) :!label _label
      (Variables|Gameplay|SetFirstNormalShot false)
      (if (not (Variables|Default|GetIsDeath)) :!label _label_2
        (CallFunction|NormalShot)
        (Audio|PlaySound2D "/Game/Retro_8Bit_Sounds/Weapons/Cues/retro_laser_gun_shoot_37_Cue.retro_laser_gun_shoot_37_Cue" 1.0 1.0 0.0 0 0)
        (goto _label))
      (else
        (Utilities|FlowControl|Delay (Variables|Default|GetBulletRate))
        (Utilities|FlowControl|Sequence
          (:then_0
            (if Pressed
              (goto _label_2)
              (else
                (goto _label_3 Reset))))
          (:then_1
            (Utilities|FlowControl|DoOnce true :!label _label_3
              (:Completed
                (Variables|Gameplay|SetFirstNormalShot true)))))))
    (else
      (goto _label_3))))

(event EventIPauseGame
  (params (Pressed :type Boolean))
  (if Pressed
    (Widget|RemovefromParent (Variables|Widget|GetGameHUD))
    (Utilities|IsValid (Variables|Widget|GetPauseGame)
      (:Is%20Valid
        (UserInterface|Viewport|AddtoViewport (Variables|Widget|GetPauseGame) 0))
      (:Is%20Not%20Valid
        (bind _returnvalue (UserInterface|CreateWidget "/Game/Astroroide/UI/WBP_PauseGame.WBP_PauseGame_C"))
        (bind _output_get (Variables|Widget|SetPauseGame _returnvalue))
        (UserInterface|Viewport|AddtoViewport _output_get 0)))
    (else
      (Widget|RemovefromParent (Variables|Widget|GetPauseGame))
      (UserInterface|Viewport|AddtoViewport (Variables|Widget|GetGameHUD) 0))))

(fn ConstructionScript)