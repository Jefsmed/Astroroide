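; Player controller for Astroroide gameplay that shows a loading screen on begin play and relays input to the controlled ship.
; Movement and firing go to the pawn through interface messages, gated by flags for match release and pause.
; The pause toggle always notifies the pawn, but freezes the game only when the player is not in a session.
; It also stores the match timer and shows the cursor at match end.
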(event Custom|EventGameplayReleased
  ;[0.4583 0.02387 0.02387] Multicast events to release controller functions when the game starts and block functions when the game ends.
  (Variables|Gameplay|SetGameplayReleased true))

(event Custom|StartLoadingScreen
  ;[1 0.9225 0] Loading screen for enter the lobby
  (Networking|SwitchHasAuthority
    (:Authority
      _)
    (:Remote
      _))
  (bind _returnvalue (UserInterface|CreateWidget "/Game/Astroroide/UI/WBP_LoadingGame.WBP_LoadingGame_C"))
  (bind _output_get (Variables|WidgetInterface|SetWBP_LoadingGame _returnvalue))
  (UserInterface|Viewport|AddtoViewport _output_get 10))

(event Custom|RemoveLoadingScreen
  ;[1 0.9225 0] Loading screen for enter the lobby
  (Widget|RemovefromParent (Variables|WidgetInterface|GetWBP_LoadingGame)))

(event Custom|EventGameplayEndMatch
  ;[0.4583 0.02387 0.02387] Multicast events to release controller functions when the game starts and block functions when the game ends.
  (Variables|Gameplay|SetGameplayReleased false)
  (Variables|Default|SetbShowMouseCursor true))

(event EventBeginPlay
  (CallFunction|StartLoadingScreen))

(event Custom|PauseGameMenu
  ;[1 1 1] PauseGame
  (if (Variables|Gameplay|GetGameplayReleased)
    (bind _bisinsession (Class|AdvancedSessionsLibrary|IsPlayerinSession (Class|AdvancedSessionsLibrary|GetUniqueNetIDfromPlayerState (Variables|Default|GetPlayerState))))
    (if _bisinsession
      (Utilities|FlowControl|FlipFlop
        (:A
          (Class|BPIInputs|IPauseGame(Message) (Pawn|GetControlledPawn) true)
          (Variables|Default|SetbShowMouseCursor true))
        (:B
          (Class|BPIInputs|IPauseGame(Message) (Pawn|GetControlledPawn) false)
          (Variables|Default|SetbShowMouseCursor true)))
      (else
        (Utilities|FlowControl|FlipFlop
          (:A
            (Game|SetGamePaused true)
            (Variables|Gameplay|SetPauseGame true)
            (Class|BPIInputs|IPauseGame(Message) (Pawn|GetControlledPawn) true)
            (Variables|Default|SetbShowMouseCursor true))
          (:B
            (Game|SetGamePaused false)
            (Variables|Gameplay|SetPauseGame false)
            (Class|BPIInputs|IPauseGame(Message) (Pawn|GetControlledPawn) false)
            (Variables|Default|SetbShowMouseCursor false)))))))

(event Input|ActionEvents|InputActionNormalShot
  (params (Key :type Key%20Structure :default "None"))
  (bind _returnvalue (Pawn|GetControlledPawn))
  (bind _gameplayreleased (Variables|Gameplay|GetGameplayReleased))
  (bind _pausegame (Variables|Gameplay|GetPauseGame))
  ;[1 1 1] Input for ship firing.
  (:Pressed
    (if _gameplayreleased
      (if (not _pausegame)
        (Class|BPIInputs|INormalShot(Message) _returnvalue true))))
  (:Released
    (if _gameplayreleased
      (if (not _pausegame)
        (Class|BPIInputs|INormalShot(Message) _returnvalue false)))))

(event Input|ActionEvents|InputActionPauseGame
  (params (Key :type Key%20Structure :default "None"))
  ;[1 1 1] PauseGame
  (:Pressed
    (if (Variables|Gameplay|GetGameplayReleased)
      (bind _bisinsession (Class|AdvancedSessionsLibrary|IsPlayerinSession (Class|AdvancedSessionsLibrary|GetUniqueNetIDfromPlayerState (Variables|Default|GetPlayerState))))
      (if _bisinsession
        (Utilities|FlowControl|FlipFlop
          (:A
            (Class|BPIInputs|IPauseGame(Message) (Pawn|GetControlledPawn) true)
            (Variables|Default|SetbShowMouseCursor true))
          (:B
            (Class|BPIInputs|IPauseGame(Message) (Pawn|GetControlledPawn) false)
            (Variables|Default|SetbShowMouseCursor true)))
        (else
          (Utilities|FlowControl|FlipFlop
            (:A
              (Game|SetGamePaused true)
              (Variables|Gameplay|SetPauseGame true)
              (Class|BPIInputs|IPauseGame(Message) (Pawn|GetControlledPawn) true)
              (Variables|Default|SetbShowMouseCursor true))
            (:B
              (Game|SetGamePaused false)
              (Variables|Gameplay|SetPauseGame false)
              (Class|BPIInputs|IPauseGame(Message) (Pawn|GetControlledPawn) false)
              (Variables|Default|SetbShowMouseCursor false))))))))

(event Input|AxisEvents|InputAxisMoveForward/Backward
  (params (AxisValue :type Float%20%28single-precision%29))
  ;[1 1 1] Basic Movements
  (if (Variables|Gameplay|GetGameplayReleased)
    (if (not (Variables|Gameplay|GetPauseGame))
      (Class|BPIInputs|IMoveForward/Backward(Message) (Pawn|GetControlledPawn) AxisValue))))

(event Input|AxisEvents|InputAxisMoveRight/Left
  (params (AxisValue :type Float%20%28single-precision%29))
  ;[1 1 1] Basic Movements
  (if (Variables|Gameplay|GetGameplayReleased)
    (if (not (Variables|Gameplay|GetPauseGame))
      (Class|BPIInputs|IMoveRight/Left(Message) (Pawn|GetControlledPawn) AxisValue))))

(fn ConstructionScript)

(fn UpdateMatchTimer
  (params (Minute :type Integer) (Second :type Integer))
  (Variables|MatchTimer|SetMatchTimerMinute Minute)
  (Variables|MatchTimer|SetMatchTimerSecond Second))

(fn GetMatchTimer
  (return (Variables|MatchTimer|GetMatchTimerMinute) (Variables|MatchTimer|GetMatchTimerSecond)))