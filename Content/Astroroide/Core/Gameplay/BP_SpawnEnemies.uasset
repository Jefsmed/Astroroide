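; Enemy spawner actor that releases BP_Enemy actors at random intervals from arrow markers around a configurable box.
; Once StartSpawnEnemies is called, a self-repeating delay capped by MaxSpawnTimer spawns each enemy at a random arrow.
; Its velocity direction comes from a re-rolled random arrow, with yaw jitter, so it can differ from the spawn arrow.
; The Construction Script sizes the box, syncs Position and Rotation arrays to Arrows, and creates the arrow components.
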(event Custom|SpawnEnemys
  (bind _arrows (Variables|SpawnPoints|GetArrows))
  (bind _returnvalue (Utilities|Array|Length _arrows))
  (bind _returnvalue_2 (- _returnvalue 1))
  (bind _returnvalue_3 (Math|Random|RandomIntegerinRange 0 _returnvalue_2))
  (bind _output (Utilities|Array|Get(acopy) _arrows _returnvalue_3))
  (bind _returnvalue_4 (Transformation|GetWorldTransform _output))
  (bind _rotation (Math|Transform|BreakTransform _returnvalue_4))
  (bind _returnvalue_5 (Game|SpawnActorfromClass "/Game/Astroroide/Core/Gameplay/BP_Enemy.BP_Enemy_C" _returnvalue_4 "Undefined" 0 0))
  (Default|ModifyVelocity _returnvalue_5 (Math|Vector|GetForwardVector (Math|Rotator|MakeRotator (.roll _rotation) (.pitch _rotation) (+ (.yaw _rotation) (Math|Random|RandomFloatinRange -3e+01 3e+01)))))
  (Utilities|FlowControl|Delay (Math|Random|RandomFloatinRange 0.3 (Variables|Default|GetMaxSpawnTimer)))
  (CallFunction|SpawnEnemys))

(event Custom|StartSpawnEnemies
  (Utilities|FlowControl|Delay (Math|Random|RandomFloatinRange 0.3 (Variables|Default|GetMaxSpawnTimer)))
  (CallFunction|SpawnEnemys))

(event EventBeginPlay)

(fn ConstructionScript
  (bind _position (Variables|SpawnPoints|GetPosition))
  (bind _returnvalue (Utilities|Array|Length _position))
  (Components|Box|SetBoxExtent (Variables|Default|GetSpawnArea) (Variables|Default|GetBox%20Extent) true)
  (Math|Integer|CompareInt (Utilities|Array|Length (Variables|SpawnPoints|GetArrows)) _returnvalue
    (:>
      (Utilities|Array|Add :TargetArray (Variables|SpawnPoints|GetPosition))
      (Utilities|Array|Add :TargetArray (Variables|SpawnPoints|GetRotation)))
    (:==
      _)
    (:<
      (for _index (range (- (Utilities|Array|Length (Variables|SpawnPoints|GetArrows)) 1) (- _returnvalue 1))
        (Utilities|Array|RemoveIndex (Variables|SpawnPoints|GetPosition) _index)
        (Utilities|Array|RemoveIndex (Variables|SpawnPoints|GetRotation) _index))))
  (for (_ _array_index) (Variables|SpawnPoints|GetArrows)
    (bind _returnvalue_2 (AddComponent|AddArrowComponent false (Math|Transform|MakeTransform (Utilities|Array|Get(acopy) (Variables|SpawnPoints|GetPosition) _array_index) (Utilities|Array|Get(acopy) (Variables|SpawnPoints|GetRotation) _array_index) "1.000000,1.000000,1.000000")))
    (Utilities|Array|SetArrayElem (Variables|SpawnPoints|GetArrows) _array_index _returnvalue_2)))