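; Game mode for an Astroroide match that spawns player spaceships and runs the match timer.
; On BeginPlay it caches player starts and gathers player controllers through a gated retry, then starts the match after a fixed delay.
; Each player possesses a color-coded ship from a DataTable at a random start, then HUDs, camera and enemy spawners are initialized.
; A self-calling delayed countdown pushes the remaining time to each player controller.
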(event Custom|StartMatchgame
  ;[0.1467 1 0.1406] Spawn Spaceship for gameplay
  (for (_array_element _array_index) (Variables|Default|GetAllPlayers)
    (bind _aspc_astroroide_gameplay (Utilities|Casting|CastToPC_AstroroideGameplay _array_element))
    (bind _returnvalue (Utilities|GetDataTableRow "/Game/Astroroide/DataTable/DT_PlayerSpaceships.DT_PlayerSpaceships" (Utilities|String|StringToName (Utilities|String|EnumtoString (Class|AstroroideController|GetSpaceshipSelected _aspc_astroroide_gameplay))))
      (:then
        (bind _returnvalue_2 (Game|SpawnActorfromClass "/Game/Astroroide/Core/Gameplay/BP_Spaceship.BP_Spaceship_C" (Transformation|GetActorTransform (Utilities|Array|Get(acopy) (Variables|Default|GetAllPlayersStart) (Math|Random|RandomIntegerinRange 0 3))) "Undefined" _array_element 0))
        (Default|ConfigureSpaceshipbyPlayerID _returnvalue_2 (Utilities|Array|Get(acopy) (Variables|Default|GetColor%20ID) _array_index) (.spaceship _returnvalue))
        (Pawn|Possess _array_element _returnvalue_2)
        (Utilities|Array|Add (Variables|Default|GetSpaceshipChars) _returnvalue_2))))
  (for _array_element_2 (Variables|Default|GetSpaceshipChars)
    (Default|CreateHUD _array_element_2))
  (bind _outactors (Actor|GetAllActorsOfClass "/Game/Astroroide/Core/Gameplay/BP_GameplayCamera.BP_GameplayCamera_C"))
  (Default|ConfigurGameplayCamera (Utilities|Array|Get(acopy) _outactors))
  (CallFunction|StartMatchgameCountdown)
  (for _array_element_3 (Variables|Default|GetAllPlayers)
    (bind _aspc_astroroide_gameplay_2 (Utilities|Casting|CastToPC_AstroroideGameplay _array_element_3))
    (Widget|RemovefromParent (Variables|/Game/Astroroide/Core/Gameplay/PC_AstroroideGameplay.PC_AstroroideGameplay_C|GetWBP_LoadingGame _aspc_astroroide_gameplay_2)))
  (bind _outactors_2 (Actor|GetAllActorsOfClass "/Game/Astroroide/Core/Gameplay/BP_SpawnEnemies.BP_SpawnEnemies_C"))
  (bind _output_get (Variables|Default|SetSpawnEnemies _outactors_2))
  (for _array_element_4 _output_get
    (Default|StartSpawnEnemies _array_element_4)))

(event Custom|GetAllPlayersConnectedToMatch
  ;[1 1 1] When starting the session, it scans the map to get all the players in the game, ending it starts looking for new players in the session and starts the timer.
  (Utilities|FlowControl|Gate false
    (:Exit
      (bind _outactors (Actor|GetAllActorsOfClass "/Script/Engine.PlayerController"))
      (if (> (Utilities|Array|Length _outactors) (Utilities|Array|Length (Variables|Default|GetAllPlayers)))
        (for _array_element _outactors
          (Utilities|Array|Add (Variables|Default|GetAllPlayers) _array_element))
        (else
          (Utilities|FlowControl|Delay 0.2)
          (CallFunction|GetAllPlayersConnectedtoMatch))))))

(event Custom|TimerVerifyAllPlayers
  ;[1 1 1] When starting the session, it scans the map to get all the players in the game, ending it starts looking for new players in the session and starts the timer.
  (Utilities|FlowControl|Delay 5.0)
  (Utilities|FlowControl|Sequence
    (:then_0
      (Utilities|FlowControl|Gate false) ; enters at Close
    )
    (:then_1
      (CallFunction|StartMatchgame))))

(event Custom|Countdown
  ;[1 1 1] Countdown
  (bind _output_get (Variables|MultiplayerTimer|SetSecond (- (Variables|MultiplayerTimer|GetSecond) 1)))
  (if (< _output_get 0)
    (Variables|MultiplayerTimer|SetSecond 59)
    (CallFunction|EventforMinute)
    (bind _output_get_2 (Variables|MultiplayerTimer|SetMinute (- (Variables|MultiplayerTimer|GetMinute) 1)))
    (if (not (< _output_get_2 0))
      (Utilities|FlowControl|Delay 1.0 :!label _label)
      (CallFunction|CountDown)
      (for _array_element (Variables|Default|GetAllPlayers)
        (bind _aspc_astroroide_gameplay (Utilities|Casting|CastToPC_AstroroideGameplay _array_element))
        (Default|UpdateCountdown _aspc_astroroide_gameplay (Variables|MultiplayerTimer|GetMinute) (Variables|MultiplayerTimer|GetSecond))))
    (else
      (goto _label))))

(event Custom|EventForMinute)

(event Custom|StartMatchgameCountdown
  (Variables|MultiplayerTimer|SetMinute 3)
  (Variables|MultiplayerTimer|SetSecond 0)
  (CallFunction|CountDown))

(event EventPostLogin
  (params (NewPlayer :type Player%20Controller%20Object%20Reference))
  (|CallParentFunction NewPlayer))

(event EventBeginPlay
  ;[1 1 1] When starting the session, it scans the map to get all the players in the game, ending it starts looking for new players in the session and starts the timer.
  (|CallParentFunction)
  (bind _outactors (Actor|GetAllActorsOfClass "/Script/Engine.PlayerStart"))
  (Variables|Default|SetAllPlayersStart _outactors)
  (CallFunction|GetAllPlayersConnectedtoMatch)
  (CallFunction|TimerVerifyAllPlayers))

(fn ConstructionScript)

(fn GetPlayerSpaceshipSelected
  (params (Controller :type PC%20Astroroide%20Gameplay%20Object%20Reference))
  (if (Utilities|Enum|Equal(Enum) (Variables|/Script/Astroroide.AstroroideController|GetSpaceshipSelected Controller) "None")
    (Variables|/Script/Astroroide.AstroroideController|SetSpaceshipSelected Controller "Fighter"))
  (return (Utilities|String|StringToName (Utilities|String|EnumtoString (Variables|/Script/Astroroide.AstroroideController|GetSpaceshipSelected Controller)))))