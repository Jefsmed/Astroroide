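; Player controller for the Astroroide online lobby that sets up the lobby UI and passes player input to the controlled pawn.
; On BeginPlay it shows a loading widget, then creates the lobby widget and removes the loading one.
; Movement axes and normal-shot press/release go to the pawn through interface messages.
; It also stores a minute/second countdown behind update and get functions.
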(event Custom|StartLoadingScreen
  ;[1 0.9225 0] Loading screen for enter the lobby
  (Networking|SwitchHasAuthority
    (:Authority
      _)
    (:Remote
      _))
  (bind _returnvalue (UserInterface|CreateWidget "/Game/Astroroide/UI/WBP_LoadingGame.WBP_LoadingGame_C"))
  (bind _output_get (Variables|WidgetInterface|SetWBP_LoadingGame _returnvalue))
  (UserInterface|Viewport|AddtoViewport _output_get 10))

(event Custom|CreateLobbyInterface
  ;[0.3854 0.3574 0.02409] Create Lobby interface
  (Networking|SwitchHasAuthority
    (:Authority
      _)
    (:Remote
      _))
  (bind _returnvalue (UserInterface|CreateWidget "/Game/Astroroide/UI/WBP_Lobby.WBP_Lobby_C" self))
  (bind _output_get (Variables|WidgetInterface|SetWBP_Lobby _returnvalue))
  (UserInterface|Viewport|AddtoViewport _output_get 0)
  (Widget|RemovefromParent (Variables|WidgetInterface|GetWBP_LoadingGame)))

(event EventBeginPlay
  (CallFunction|StartLoadingScreen)
  (CallFunction|CreateLobbyInterface))

(event Input|ActionEvents|InputActionNormalShot
  (params (Key :type Key%20Structure))
  (bind _returnvalue (Pawn|GetControlledPawn))
  (:Pressed
    (Class|BPIInputs|INormalShot(Message) _returnvalue true))
  (:Released
    (Class|BPIInputs|INormalShot(Message) _returnvalue false)))

(event Input|AxisEvents|InputAxisMoveForward/Backward
  (params (AxisValue :type Float%20%28single-precision%29))
  (Class|BPIInputs|IMoveForward/Backward(Message) (Pawn|GetControlledPawn) AxisValue))

(event Input|AxisEvents|InputAxisMoveRight/Left
  (params (AxisValue :type Float%20%28single-precision%29))
  (Class|BPIInputs|IMoveRight/Left(Message) (Pawn|GetControlledPawn) AxisValue))

(fn ConstructionScript)

(fn UpdateCountdown
  (params (Minute :type Integer) (Second :type Integer))
  (Variables|Default|SetMinute Minute)
  (Variables|Default|SetSecond Second))

(fn GetCountdown
  (return (Variables|Default|GetMinute) (Variables|Default|GetSecond)))