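; BP_SpaceshipLobby shows the local player's selected spaceship in the online lobby.
; On BeginPlay it reads the selection from PC_AstroroideLobby and uses the enum name as the row key into DT_PlayerSpaceships.
; It applies that row's skeletal mesh, then sets the controller's ColorID material on the player material slot.
; A RotateCamera timeline that would yaw the SpawnBullet component is present but never runs.
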(event EventBeginPlay
  (bind _aspc_astroroide_lobby (Utilities|Casting|CastToPC_AstroroideLobby (Game|GetPlayerController 0)))
  (bind _returnvalue (Utilities|GetDataTableRow "/Game/Astroroide/DataTable/DT_PlayerSpaceships.DT_PlayerSpaceships" (Utilities|String|StringToName (Utilities|String|EnumtoString (Class|AstroroideController|GetSpaceshipSelected _aspc_astroroide_lobby))))
    (:then
      (Components|SkeletalMesh|SetSkeletalMeshAsset (Variables|Character|GetMesh) (Utilities|Struct|BreakSPlayerSpaceShips (.spaceship _returnvalue)))
      (Rendering|Material|SetMaterialbyName (Variables|Character|GetMesh) "M_PlayerMaterial" (Variables|/Game/Astroroide/Core/OnlineLobby/PC_AstroroideLobby.PC_AstroroideLobby_C|GetColorID _aspc_astroroide_lobby)))))

(fn ConstructionScript)