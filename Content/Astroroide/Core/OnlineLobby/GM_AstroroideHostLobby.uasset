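; Lobby game mode for Astroroide that assigns player colors and runs the timer before the match starts.
; Each login adds the player to a list and reassigns every lobby controller's ColorID by its index.
; A self-calling countdown with one-second delays, started on BeginPlay, pushes minutes and seconds to each lobby controller.
; When time runs out, it removes all widgets and server-travels to L_Gameplay.
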(event Custom|Countdown
  ;[1 1 1] Comment
  (bind _output_get (Variables|Default|SetSecond (- (Variables|Default|GetSecond) 1)))
  (if (< _output_get 0)
    (Variables|Default|SetSecond 59)
    (bind _output_get_2 (Variables|Default|SetMinute (- (Variables|Default|GetMinute) 1)))
    (if (< _output_get_2 0)
      (Variables|Default|SetMinute 0)
      (Variables|Default|SetSecond 0)
      (Viewport|RemoveAllWidgets)
      (Development|ExecuteConsoleCommand "servertravel L_Gameplay" (Game|GetPlayerController 0))
      (else
        (Utilities|FlowControl|Delay 1.0 :!label _label)
        (CallFunction|CountDown)
        (for _array_element (Variables|Default|GetAllPlayers)
          (bind _aspc_astroroide_lobby (Utilities|Casting|CastToPC_AstroroideLobby _array_element))
          (Default|UpdateCountdown _aspc_astroroide_lobby (Variables|Default|GetMinute) (Variables|Default|GetSecond)))))
    (else
      (goto _label))))

(event EventBeginPlay
  (CallFunction|CountDown))

(event EventPostLogin
  (params (NewPlayer :type Player%20Controller%20Object%20Reference))
  (Utilities|Array|Add (Variables|Default|GetAllPlayers) NewPlayer)
  (for (_array_element _array_index) (Variables|Default|GetAllPlayers)
    (bind _aspc_astroroide_lobby (Utilities|Casting|CastToPC_AstroroideLobby _array_element))
    (Variables|/Game/Astroroide/Core/OnlineLobby/PC_AstroroideLobby.PC_AstroroideLobby_C|SetColorID _aspc_astroroide_lobby (Utilities|Array|Get(acopy) (Variables|Default|GetColor%20ID) _array_index))))

(fn ConstructionScript)