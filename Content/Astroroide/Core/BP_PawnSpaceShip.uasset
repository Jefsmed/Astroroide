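; Player spaceship pawn that moves on a horizontal plane, turns its mesh to face the travel direction and fires bullets.
; Axis input events store the last direction and trigger acceleration or deceleration.
; Gates, DoOnces and short Delay loops, rather than Tick, ramp a velocity factor up and down, so the ship coasts when input stops.
; The shot event spawns BP_Bullet at the Arrow on a repeating delay while Pressed is true.
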(event EventBeginPlay)

(event Collision|EventActorBeginOverlap
  (params (OtherActor :type Actor%20Object%20Reference)))

(event EventTick
  (params (DeltaSeconds :type Float%20%28single-precision%29)))

(event Custom|StartAcceleration
  ;[1 1 1] Aceleração
  (Utilities|FlowControl|DoOnce false
    (:Completed
      (Utilities|FlowControl|Sequence
        (:then_0
          (Utilities|FlowControl|Delay 0.01)
          (Utilities|FlowControl|Gate true :!label _label
            (:Exit
              (if (Math|Float|NearlyEqual(Float) (Variables|Default|GetCurrentAcceleration) (Variables|Default|GetAcceleration) 0.01)
                (Variables|Default|SetCurrentAcceleration (Variables|Default|GetAcceleration))
                (else
                  (Utilities|FlowControl|Delay 0.01)
                  (Variables|Default|SetCurrentAcceleration (+ (Variables|Default|GetCurrentAcceleration) 0.1))
                  (Utilities|FlowControl|Sequence
                    (:then_0
                      _)
                    (:then_1
                      (goto _label)))))
              (if (or (!= (Variables|AxisMapping|GetRight%20Left%20Axis%20Value) 0.0) (!= (Variables|AxisMapping|GetForward%20Backward%20Axis%20Value) 0.0)) :!label _label_2
                (Utilities|FlowControl|Sequence
                  (:then_0
                    (Utilities|FlowControl|Delay 0.01)
                    (goto _label_2))
                  (:then_1
                    _)))
              (Utilities|FlowControl|Sequence
                (:then_0
                  (Class|PawnSpaceShip|MoveForwardBackward (* (Variables|Default|GetDirectionForwardBackward) (* (Variables|Default|GetVelocity) (/ (Variables|Default|GetCurrentAcceleration) (Variables|Default|GetAcceleration))))))
                (:then_1
                  (Class|PawnSpaceShip|MoveRightLeft (* (Variables|Default|GetDirectionRightLeft) (* (Variables|Default|GetVelocity) (/ (Variables|Default|GetCurrentAcceleration) (Variables|Default|GetAcceleration))))))))))
        (:then_1
          (goto _label Open))
        (:then_2
          (Utilities|FlowControl|Gate true) ; enters at Close
        )
        (:then_3
          (Utilities|FlowControl|DoOnce false) ; enters at Reset
        )))))

(event Custom|StartDesacelaration
  ;[1 1 1] Aceleração
  (if (and (== (Variables|AxisMapping|GetRight%20Left%20Axis%20Value) 0.0) (== (Variables|AxisMapping|GetForward%20Backward%20Axis%20Value) 0.0))
    (Utilities|FlowControl|DoOnce false
      (:Completed
        (Utilities|FlowControl|Sequence
          (:then_0
            (Utilities|FlowControl|DoOnce false) ; enters at Reset
          )
          (:then_1
            (Utilities|FlowControl|Gate true) ; enters at Close
          )
          (:then_2
            (Utilities|FlowControl|Delay 0.01)
            (Utilities|FlowControl|Gate true :!label _label
              (:Exit
                (if (Math|Float|NearlyEqual(Float) (Variables|Default|GetCurrentAcceleration) 0.0 0.01)
                  (Variables|Default|SetCurrentAcceleration 0.0)
                  (else
                    (Utilities|FlowControl|Delay 0.01)
                    (Variables|Default|SetCurrentAcceleration (- (Variables|Default|GetCurrentAcceleration) 0.1))
                    (Utilities|FlowControl|Sequence
                      (:then_0
                        _)
                      (:then_1
                        (goto _label)))))
                (if (or (!= (Variables|AxisMapping|GetRight%20Left%20Axis%20Value) 0.0) (!= (Variables|AxisMapping|GetForward%20Backward%20Axis%20Value) 0.0)) :!label _label_2
                  (Utilities|FlowControl|Sequence
                    (:then_0
                      (Utilities|FlowControl|Delay 0.01)
                      (goto _label_2))
                    (:then_1
                      _)))
                (Utilities|FlowControl|Sequence
                  (:then_0
                    (Class|PawnSpaceShip|MoveForwardBackward (* (Variables|Default|GetDirectionForwardBackward) (* (Variables|Default|GetVelocity) (/ (Variables|Default|GetCurrentAcceleration) (Variables|Default|GetAcceleration))))))
                  (:then_1
                    (Class|PawnSpaceShip|MoveRightLeft (* (Variables|Default|GetDirectionRightLeft) (* (Variables|Default|GetVelocity) (/ (Variables|Default|GetCurrentAcceleration) (Variables|Default|GetAcceleration))))))))))
          (:then_3
            (goto _label Open)))))))

(event EventIMoveForward/Backward
  (params (AxisValue :type Float%20%28double-precision%29))
  (bind _output_get (Variables|AxisMapping|SetForward%20Backward%20Axis%20Value AxisValue))
  (Utilities|FlowControl|Sequence
    (:then_0
      (Utilities|FlowControl|Gate true :!label _label
        (:Exit
          (Utilities|FlowControl|Sequence
            (:then_0
              (if (!= (Variables|AxisMapping|GetForward%20Backward%20Axis%20Value) 0.0)
                (Variables|Default|SetDirectionForwardBackward (Variables|AxisMapping|GetForward%20Backward%20Axis%20Value))
                (if (== (Variables|AxisMapping|GetRight%20Left%20Axis%20Value) 0.0)
                  (Variables|Default|SetDirectionRightLeft 0.0))))
            (:then_1
              (CallFunction|StartAcceleration)
              (Transformation|SetWorldRotation (Variables|Default|GetMesh) (Math|Conversions|RotationFromXVector (Math|Vector|MakeVector (Variables|Default|GetDirectionForwardBackward) (Variables|Default|GetDirectionRightLeft) 0.0)) false false))))))
    (:then_1
      (Math|Float|CompareFloat _output_get 0.0
        (:>
          (goto _label Open))
        (:==
          (Utilities|FlowControl|Sequence
            (:then_0
              (goto _label Close))
            (:then_1
              (CallFunction|StartDesacelaration))))
        (:<
          (goto _label Open))))))

(event EventIMoveRight/Left
  (params (AxisValue :type Float%20%28double-precision%29))
  (bind _output_get (Variables|AxisMapping|SetRight%20Left%20Axis%20Value AxisValue))
  (Utilities|FlowControl|Sequence
    (:then_0
      (Utilities|FlowControl|Gate true :!label _label
        (:Exit
          (Utilities|FlowControl|Sequence
            (:then_0
              (if (!= (Variables|AxisMapping|GetRight%20Left%20Axis%20Value) 0.0)
                (Variables|Default|SetDirectionRightLeft (Variables|AxisMapping|GetRight%20Left%20Axis%20Value))
                (if (== (Variables|AxisMapping|GetForward%20Backward%20Axis%20Value) 0.0)
                  (Variables|Default|SetDirectionForwardBackward 0.0))))
            (:then_1
              (CallFunction|StartAcceleration)
              (Transformation|SetWorldRotation (Variables|Default|GetMesh) (Math|Conversions|RotationFromXVector (Math|Vector|MakeVector (Variables|Default|GetDirectionForwardBackward) (Variables|Default|GetDirectionRightLeft) 0.0)) false false))))))
    (:then_1
      (Math|Float|CompareFloat _output_get 0.0
        (:>
          (goto _label Open))
        (:==
          (Utilities|FlowControl|Sequence
            (:then_0
              (goto _label Close))
            (:then_1
              (CallFunction|StartDesacelaration))))
        (:<
          (goto _label Open))))))

(event EventINormalShot
  (params (Pressed :type Boolean))
  (if Pressed :!label _label
    (Game|SpawnActorfromClass "/Game/Astroroide/Core/BP_Bullet.BP_Bullet_C" (Transformation|GetWorldTransform (Variables|Default|GetArrow)) "Undefined" 0 (Transformation|GetWorldRotation (Variables|Default|GetMesh)) 0)
    (Utilities|FlowControl|Delay 0.2)
    (goto _label)))

(fn ConstructionScript
  (Components|SkeletalMesh|SetSkeletalMeshAsset (Variables|Default|GetMesh) (Variables|Mesh|GetSpaceshipMesh)))