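; Gameplay game mode for Astroroide that spawns and assigns each player's spaceship as play begins.
; It shows a loading widget, waits briefly, then gathers all player controllers.
; Each gets a BP_Spaceship at a random PlayerStart (repeats possible), configured from the hardcoded "Destroyer" data table row and a player-index material, then possesses it.
; Ship HUDs are created after the spawn loop, then the loading widget is removed.
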(event Custom|SpawnSpaceships
  (bind _outactors (Actor|GetAllActorsOfClass "/Script/Engine.PlayerStart"))
  (for (_array_element _array_index) (Variables|Default|GetAllPlayers)
    (bind _aspc_astroroide (Utilities|Casting|CastToPC_Astroroide _array_element))
    (bind _returnvalue (Utilities|GetDataTableRow "/Game/Astroroide/DataTable/DT_PlayerSpaceships.DT_PlayerSpaceships" "Destroyer")
      (:then
        (bind _returnvalue_2 (Game|SpawnActorfromClass :Class "/Game/Astroroide/Core/BP_Spaceship.BP_Spaceship_C" :SpawnTransform (Transformation|GetActorTransform (Utilities|Array|Get(acopy) _outactors (Math|Random|RandomIntegerinRange 0 3))) :CollisionHandlingOverride "Undefined" :Owner _array_element :Instigator 0))
        (Default|ConfigureSpaceshipbyPlayerID _returnvalue_2 (Utilities|Select :Index _array_index :Option%200 "/Game/Astroroide/Materials/MI_PlayerID_00.MI_PlayerID_00" :Option%201 "/Game/Astroroide/Materials/MI_PlayerID_01.MI_PlayerID_01" :Option%202 "/Game/Astroroide/Materials/MI_PlayerID_02.MI_PlayerID_02" :Option%203 "/Game/Astroroide/Materials/MI_PlayerID_03.MI_PlayerID_03") (.spaceship _returnvalue))
        (Pawn|Possess _array_element _returnvalue_2)
        (Utilities|Array|Add (Variables|Default|GetSpaceshipChars) _returnvalue_2))))
  (for _array_element_2 (Variables|Default|GetSpaceshipChars)
    (Default|CreateHUD _array_element_2))
  (Widget|RemovefromParent (Variables|Default|GetWBP_LoadingGame)))

(event EventBeginPlay
  (bind _returnvalue (UserInterface|CreateWidget "/Game/Astroroide/UI/WBP_LoadingGame.WBP_LoadingGame_C"))
  (bind _output_get (Variables|Default|SetWBP_LoadingGame _returnvalue))
  (UserInterface|Viewport|AddtoViewport _output_get 10)
  (Utilities|FlowControl|Delay 3.0)
  (bind _outactors (Actor|GetAllActorsOfClass "/Script/Engine.PlayerController"))
  (Variables|Default|SetAllPlayers _outactors)
  (CallFunction|SpawnSpaceships))

(event EventTick
  (params (DeltaSeconds :type Float%20%28single-precision%29)))

(fn ConstructionScript)