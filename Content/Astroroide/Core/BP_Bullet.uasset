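; BP_Bullet is a projectile that damages Enemy actors it overlaps.
; The MovifyVelocity event sets the ProjectileMovement velocity to a given forward vector scaled by its initial speed.
; Capsule overlaps filter for Enemy and apply the Damage value, crediting the bullet's owner as causer and that owner's instigator controller as instigator.
; The graph does not destroy the bullet on a hit.
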(event OnComponentBeginOverlap(Capsule)
  (params (OverlappedComponent :type Primitive%20Component%20Object%20Reference) (OtherActor :type Actor%20Object%20Reference) (OtherComp :type Primitive%20Component%20Object%20Reference) (OtherBodyIndex :type Integer) (bFromSweep :type Boolean) (SweepResult :type Hit%20Result%20Structure%20%28by%20ref%29))
  (bind _returnvalue (Components|GetOwner))
  (Utilities|Casting|CastToEnemy OtherActor)
  (Game|Damage|ApplyDamage OtherActor (Math|Conversions|ToFloat(Integer) (Variables|Default|GetDamage)) (Game|GetInstigatorController _returnvalue) _returnvalue))

(event Custom|MovifyVelocity
  (params (Forward%20vector :type Vector))
  (bind _projectilemovement (Variables|Default|GetProjectileMovement))
  (Variables|/Script/Engine.MovementComponent|SetVelocity _projectilemovement (* Forward%20vector (Variables|/Script/Engine.ProjectileMovementComponent|GetInitialSpeed _projectilemovement))))

(fn ConstructionScript)