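; Base enemy projectile actor for Astroroide that acts as an asteroid or, when flagged as an alien, skips the random spin and speed setup.
; Projectile and rotating movement drive it, ModifyVelocity aims it along a given forward vector, and the construction script applies a configurable mesh.
; Any damage caused by BP_Spaceship awards that ship points and destroys the enemy.
; Overlapping a SpaceshipChar damages that character and destroys the enemy.
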(event OnComponentBeginOverlap(Capsule)
  (params (OverlappedComponent :type Primitive%20Component%20Object%20Reference) (OtherActor :type Actor%20Object%20Reference) (OtherComp :type Primitive%20Component%20Object%20Reference) (OtherBodyIndex :type Integer) (bFromSweep :type Boolean) (SweepResult :type Hit%20Result%20Structure%20%28by%20ref%29))
  (Utilities|Casting|CastToSpaceshipChar OtherActor)
  (Game|Damage|ApplyDamage OtherActor 1.0 0 0)
  (Actor|DestroyActor))

(event Custom|ModifyVelocity
  (params (ForwardVector :type Vector))
  (bind _projectilemovement (Variables|Default|GetProjectileMovement))
  (Variables|/Script/Engine.MovementComponent|SetVelocity _projectilemovement (* ForwardVector (Variables|/Script/Engine.ProjectileMovementComponent|GetInitialSpeed _projectilemovement))))

(event EventBeginPlay
  (bind _returnvalue (Math|Random|RandomFloatinRange 5e+02 1.5e+03))
  (bind _projectilemovement (Variables|Default|GetProjectileMovement))
  (Variables|Default|SetPointsForDestroyingIt 10)
  (if (not (Variables|Default|GetIsAlien))
    (Utilities|FlowControl|Sequence
      (:then_0
        (Variables|/Script/Engine.RotatingMovementComponent|SetRotationRate (Variables|Default|GetRotatingMovement) (Math|Rotator|MakeRotator (Math|Random|RandomFloatinRange -1e+02 1e+02) (Math|Random|RandomFloatinRange -1e+02 1e+02) (Math|Random|RandomFloatinRange -1e+02 1e+02))))
      (:then_1
        (Variables|/Script/Engine.ProjectileMovementComponent|SetInitialSpeed _projectilemovement _returnvalue)
        (Variables|/Script/Engine.ProjectileMovementComponent|SetMaxSpeed _projectilemovement _returnvalue)))))

(event Game|Damage|EventAnyDamage
  (params (Damage :type Float%20%28single-precision%29) (DamageType :type Damage%20Type%20Object%20Reference) (InstigatedBy :type Controller%20Object%20Reference) (DamageCauser :type Actor%20Object%20Reference))
  (bind _asbp_spaceship (Utilities|Casting|CastToBP_Spaceship DamageCauser))
  (Variables|/Game/Astroroide/Core/BP_Spaceship.BP_Spaceship_C|SetPoints _asbp_spaceship (+ (Variables|/Game/Astroroide/Core/BP_Spaceship.BP_Spaceship_C|GetPoints _asbp_spaceship) (Variables|Default|GetPointsForDestroyingIt)))
  (Actor|DestroyActor))

(fn ConstructionScript
  (Components|StaticMesh|SetStaticMesh (Variables|Default|GetMesh) (Variables|Default|GetNew%20Mesh)))