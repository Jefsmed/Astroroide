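; BP_SpaceshipSelectOnline is an actor supporting online spaceship selection and lobby camera setup in Astroroide.
; ConfigureLobbyCamera uses a DoOnce to pass its owning PC_AstroroideGameplay controller to the first BP_LobbyCamera found in the level.
; GetPlayerSpaceshipSelected returns a controller's ship choice as a Name converted from the enum, first writing Fighter to the controller if none is selected.
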(event Custom|ConfigureLobbyCamera
  ;[1 0.9225 0] Configure Camera In lobby map
  (Networking|SwitchHasAuthority
    (:Authority
      _)
    (:Remote
      _))
  (Utilities|FlowControl|DoOnce false
    (:Completed
      (bind _outactors (Actor|GetAllActorsOfClass "/Game/Astroroide/Core/BP_LobbyCamera.BP_LobbyCamera_C"))
      (Default|ConfigureCamera (Utilities|Array|Get(acopy) _outactors) (.AsPC%20Astroroide (Utilities|Casting|CastToPC_AstroroideGameplay (Components|GetOwner)))))))

(event EventBeginPlay)

(fn ConstructionScript)

(fn GetPlayerSpaceshipSelected
  (params (Controller :type PC%20Astroroide%20Gameplay%20Object%20Reference))
  (if (Utilities|Enum|Equal(Enum) (Variables|/Script/Astroroide.AstroroideController|GetSpaceshipSelected Controller) "None")
    (Variables|/Script/Astroroide.AstroroideController|SetSpaceshipSelected Controller "Fighter"))
  (return (Utilities|String|StringToName (Utilities|String|EnumtoString (Variables|/Script/Astroroide.AstroroideController|GetSpaceshipSelected Controller)))))