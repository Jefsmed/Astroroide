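; Main menu camera actor that becomes the view target and drives the menu flow between main, spaceship selection and multiplayer screens.
; Timelines slide the camera along per-transition splines, then open the matching widget on finish.
; Start events store the chosen ship in the game instance, fade out, then load Gameplay or a listen-server Lobby.
; The construction script previews the camera along flagged splines and can align their endpoints.
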(event Custom|Open%20Main%20Menu
  ;[1 0.9225 0] Open Main Menu Game
  (bind _returnvalue (UserInterface|CreateWidget "/Game/Astroroide/UI/WBP_MainMenu.WBP_MainMenu_C" (CallFunction|GetCurrentController)))
  (UserInterface|Viewport|AddtoViewport _returnvalue 0)
  (EventDispatchers|BindEventtoSelectSinglePlay _returnvalue (delegate Custom|CustomEvent_1))
  (EventDispatchers|AssignSelectMultiplayer _returnvalue (delegate Custom|CustomEvent_2)))

(event Custom|MainMenuToSelectSpaceshp
  (params (Multiplayer :type Boolean))
  ;[0.08632 0.5885 0.08276] Single player camera animation
  (bind _alpha (Timeline|Anim_MainMenuToSinglePlay PlayFromStart)
    (:Update
      (CallFunction|CameraAnimation (Variables|Default|GetSP_MainMenuToSinglePlay) _alpha))
    (:Finished
      (CallFunction|OpenSpaceshipSelection Multiplayer))))

(event Custom|StartSinglePlayer
  ;[0.08632 0.5885 0.08276] Start Single player Mode
  (bind _asgi_astroroide (Utilities|Casting|CastToGI_Astroroide (Game|GetGameInstance)))
  (Variables|/Game/Astroroide/Core/GI_Astroroide.GI_Astroroide_C|SetSpaceshipSelected _asgi_astroroide (Variables|/Script/Astroroide.AstroroideController|GetSpaceshipSelected (.AsAstroroide%20Controller (Utilities|Casting|CastToAstroroideController (CallFunction|GetCurrentController)))))
  (bind _returnvalue (UserInterface|CreateWidget "/Game/Astroroide/UI/WBP_Fade.WBP_Fade_C"))
  (Default|StartFadeOut _returnvalue)
  (UserInterface|Viewport|AddtoViewport _returnvalue 0)
  (EventDispatchers|AssignFinishFadeOut _returnvalue (delegate Custom|FinishFade_Out_Event)))

(event Custom|MultiplayerOnlineToSelectSpaceship
  ;[0.09237 0.2 0.9062] Multiplayer Camera Animation
  (bind _alpha (Timeline|Anim_MultiplayerToSelectSpaceship PlayFromStart)
    (:Update
      (CallFunction|CameraAnimation (Variables|Default|GetSP_MultiplayerToSelectSpaceship) _alpha))
    (:Finished
      (CallFunction|OpenSpaceshipSelection true))))

(event Custom|SelectSpaceshipToMultiplayer
  ;[0.09237 0.2 0.9062] Multiplayer Camera Animation
  (bind _alpha (Timeline|Anim_MainMenuToMultiplayer PlayFromStart)
    (:Update
      (CallFunction|CameraAnimation (Variables|Default|GetSP_MainMenuToMultiplayer) _alpha))
    (:Finished
      (CallFunction|OpenMultiplayerMode))))

(event Custom|StartMultiplayerOnline
  ;[0.04645 0.05452 0.4955] Start Multiplayer mode - jump to Lobby map
  (bind _asgi_astroroide (Utilities|Casting|CastToGI_Astroroide (Game|GetGameInstance)))
  (Variables|/Game/Astroroide/Core/GI_Astroroide.GI_Astroroide_C|SetSpaceshipSelected _asgi_astroroide (Variables|/Script/Astroroide.AstroroideController|GetSpaceshipSelected (.AsAstroroide%20Controller (Utilities|Casting|CastToAstroroideController (CallFunction|GetCurrentController)))))
  (if (Networking|IsServer)
    (Variables|/Game/Astroroide/Core/GI_Astroroide.GI_Astroroide_C|SetIsLobbyMap _asgi_astroroide true)
    (else
      (Variables|/Game/Astroroide/Core/GI_Astroroide.GI_Astroroide_C|SetSpaceshipSelected _asgi_astroroide "Fighter")))
  (bind _returnvalue (UserInterface|CreateWidget "/Game/Astroroide/UI/WBP_Fade.WBP_Fade_C"))
  (Default|StartFadeOut _returnvalue)
  (UserInterface|Viewport|AddtoViewport _returnvalue 0)
  (EventDispatchers|AssignFinishFadeOut _returnvalue (delegate Custom|CustomEvent)))

(event Custom|FinishFade_Out_Event
  ;[0.08632 0.5885 0.08276] Start Single player Mode
  (bind _returnvalue (UserInterface|CreateWidget "/Game/Astroroide/UI/WBP_LoadingGame.WBP_LoadingGame_C"))
  (UserInterface|Viewport|AddtoViewport _returnvalue 10)
  (Game|OpenLevel(byObjectReference) "/Game/Maps/L_Gameplay.L_Gameplay"))

(event Custom|CustomEvent_0
  ;[0.09237 0.2 0.9062] Open Multiplayer Online - Widget
  (CallFunction|MultiplayerOnlinetoSelectSpaceship)
  (CallFunction|StartMultiplayerOnline))

(event Custom|MultiplayerToMainMenu
  ;[0.09237 0.2 0.9062] Multiplayer Camera Animation
  (bind _alpha (Timeline|Anim_MultiplayerToMainMenu PlayFromStart)
    (:Update
      (CallFunction|CameraAnimation (Variables|Default|GetSP_MultiplayerToMainMenu) _alpha))
    (:Finished
      (CallFunction|OpenMainMenu))))

(event Custom|Open%20Multiplayer%20Online
  ;[0.09237 0.2 0.9062] Open Multiplayer Online - Widget
  (bind _returnvalue (UserInterface|CreateWidget "/Game/Astroroide/UI/WBP_MultiplayerOnline.WBP_MultiplayerOnline_C" (CallFunction|GetCurrentController) self))
  (UserInterface|Viewport|AddtoViewport _returnvalue 0)
  (EventDispatchers|BindEventtoSigninSession _returnvalue (delegate Custom|CustomEvent_0)))

(event Custom|SinglePlayerToMainMenu
  ;[0.08632 0.5885 0.08276] Single player camera animation
  (bind _alpha (Timeline|Anim_SinglePlayToMainMenu PlayFromStart)
    (:Update
      (CallFunction|CameraAnimation (Variables|Default|GetSP_SinglePlayerToMainMenu) _alpha))
    (:Finished
      (CallFunction|OpenMainMenu))))

(event Custom|CustomEvent_1
  ;[1 0.9225 0] Open Main Menu Game
  (CallFunction|MainMenutoSelectSpaceshp false))

(event Custom|OpenSpaceshipSelection
  (params (Multiplayer :type Boolean))
  (bind _spaceshipselection (Variables|Default|GetSpaceshipSelection))
  ;[1 0.9225 0] Open menu Spaceship selection
  (bind _returnvalue (UserInterface|CreateWidget "/Game/Astroroide/UI/WBP_SpaceshipSelection.WBP_SpaceshipSelection_C" (CallFunction|GetCurrentController) (Variables|Default|GetSpaceshipSelection) Multiplayer))
  (bind _output_get (Variables|/Game/Astroroide/Core/BP_SpaceShipSelect.BP_SpaceShipSelect_C|SetWBP_SpaceshipSelection _spaceshipselection _returnvalue))
  (Default|EnterSelectSpaceship _spaceshipselection)
  (UserInterface|Viewport|AddtoViewport _output_get 0)
  (EventDispatchers|AssignBacktoMainMenu (Variables|Default|GetSpaceshipSelection) (EventDispatchers|CreateEvent :!event Custom|SinglePlayerToMainMenu))
  (EventDispatchers|AssignSelectedSpaceshiptoSinglePlayer _output_get (EventDispatchers|CreateEvent :!event Custom|StartSinglePlayer))
  (EventDispatchers|AssignSelectedSpaceshiptoMultiplayer _output_get (EventDispatchers|CreateEvent :!event Custom|SelectSpaceshipToMultiplayer)))

(event Custom|CustomEvent
  ;[0.04645 0.05452 0.4955] Start Multiplayer mode - jump to Lobby map
  (bind _returnvalue (UserInterface|CreateWidget "/Game/Astroroide/UI/WBP_LoadingGame.WBP_LoadingGame_C"))
  (UserInterface|Viewport|AddtoViewport _returnvalue 10)
  (Game|OpenLevel(byObjectReference) "/Game/Maps/L_Lobby.L_Lobby" true "listen"))

(event Custom|Open%20Multiplayer%20Mode
  ;[0.0357 0.4694 0.9792] Open Multiplayer mode - Widget
  (bind _returnvalue (UserInterface|CreateWidget "/Game/Astroroide/UI/WBP_MultiplayerSelect.WBP_MultiplayerSelect_C" (CallFunction|GetCurrentController)))
  (UserInterface|Viewport|AddtoViewport _returnvalue 0)
  (EventDispatchers|AssignBacktoMainMenu _returnvalue (EventDispatchers|CreateEvent :!event Custom|MultiplayerToMainMenu))
  (EventDispatchers|BindEventtoMultiOnlineSelected _returnvalue (EventDispatchers|CreateEvent :!event Custom|Open%20Multiplayer%20Online)))

(event Custom|CustomEvent_2
  ;[1 0.9225 0] Open Main Menu Game
  (CallFunction|MainMenutoSelectSpaceshp true))

(event EventBeginPlay
  ;[0.04645 0.05452 0.4955] Begin Play - Set view camera
  (Game|Player|SetViewTargetwithBlend (CallFunction|GetCurrentController) self 0.0 "VTBlend_Linear" 0.0 false))

(fn ConstructionScript
  (bind _sp_mainmenutosingleplay (Variables|Default|GetSP_MainMenuToSinglePlay))
  (bind _sp_mainmenutomultiplayer (Variables|Default|GetSP_MainMenuToMultiplayer))
  (bind _sp_singleplayertomainmenu (Variables|Default|GetSP_SinglePlayerToMainMenu))
  (bind _sp_multiplayertomainmenu (Variables|Default|GetSP_MultiplayerToMainMenu))
  (bind (_initial_position _end_position) (CallFunction|SplineStartPositionandEndPosition _sp_multiplayertomainmenu "Local"))
  (bind (_initial_position_2 _end_position_2) (CallFunction|SplineStartPositionandEndPosition _sp_mainmenutosingleplay "Local"))
  (bind (_initial_position_3 _end_position_3) (CallFunction|SplineStartPositionandEndPosition _sp_mainmenutomultiplayer "Local"))
  (bind (_initial_position_4 _end_position_4) (CallFunction|SplineStartPositionandEndPosition _sp_singleplayertomainmenu "Local"))
  ;[1 1 1] Main menu to single player configure camera trail
  (if (Variables|Default|1-SinglePlay|Get1%20-%20MainMenuToSinglePlay)
    (CallFunction|CameraAnimation (Variables|Default|GetSP_MainMenuToSinglePlay) (Variables|Default|1-SinglePlay|Get1%20-%20SinglePlayerDistance))
    (if (Variables|Default|1-SinglePlay|Get1%20-%20ConfigurePositions)
      (CallFunction|AjustSplineStartPositionandEndPosition (Variables|Default|GetSP_MainMenuToSinglePlay) (Variables|Default|1-SinglePlay|Get1%20-%20MainMenuPosition) (Variables|Default|1-SinglePlay|Get1%20-%20SinglePlayPosition) "Local"))
    (Variables|Default|1-SinglePlay|Set1%20-%20MainMenuPosition _initial_position_2)
    (Variables|Default|1-SinglePlay|Set1%20-%20SinglePlayPosition _end_position_2)
    (else
      ;[1 1 1] Main menu to multiplayer configure camera trail
      (if (Variables|Default|2-Multiplayer|Get2%20-%20MainMenuToMultplayer)
        (CallFunction|CameraAnimation (Variables|Default|GetSP_MainMenuToMultiplayer) (Variables|Default|2-Multiplayer|Get2%20-%20MultiplayerDistance))
        (if (Variables|Default|2-Multiplayer|Get2%20-%20ConfigurePositions)
          (CallFunction|AjustSplineStartPositionandEndPosition (Variables|Default|GetSP_MainMenuToMultiplayer) (Variables|Default|2-Multiplayer|Get2%20-%20MainMenuPosition) (Variables|Default|2-Multiplayer|Get2%20-%20MultiplayerPosition) "Local"))
        (Variables|Default|2-Multiplayer|Set2%20-%20MainMenuPosition _initial_position_3)
        (Variables|Default|2-Multiplayer|Set2%20-%20MultiplayerPosition _end_position_3)
        (else
          ;[1 1 1] Single player back to main menu configure camera trail
          (if (Variables|Default|1-SinglePlay|1.1-BackToMainMenu|Get1%20-%20SinglePlayToMainMenu)
            (CallFunction|CameraAnimation (Variables|Default|GetSP_SinglePlayerToMainMenu) (Variables|Default|1-SinglePlay|1.1-BackToMainMenu|Get1%20-%20_SinglePlayerDistance))
            (if (Variables|Default|1-SinglePlay|1.1-BackToMainMenu|Get1%20-%20_ConfigurePositions)
              (CallFunction|AjustSplineStartPositionandEndPosition (Variables|Default|GetSP_SinglePlayerToMainMenu) (Variables|Default|1-SinglePlay|1.1-BackToMainMenu|Get1%20-%20_SinglePlayPosition) (Variables|Default|1-SinglePlay|1.1-BackToMainMenu|Get1%20-%20_MainMenuPosition) "Local"))
            (Variables|Default|1-SinglePlay|1.1-BackToMainMenu|Set1%20-%20_SinglePlayPosition _initial_position_4)
            (Variables|Default|1-SinglePlay|1.1-BackToMainMenu|Set1%20-%20_MainMenuPosition _end_position_4)
            (else
              ;[1 1 1] Multiplayer back to main menu camera animation
              (if (Variables|Default|2-Multiplayer|2.1-MultplayerToMainMenu|Get2%20-%20MultplayerToMainMenu)
                (CallFunction|CameraAnimation (Variables|Default|GetSP_MultiplayerToMainMenu) (Variables|Default|2-Multiplayer|2.1-MultplayerToMainMenu|Get2%20-%20_MultiplayerDistance))
                (if (Variables|Default|2-Multiplayer|2.1-MultplayerToMainMenu|Get2%20-%20_ConfigurePositions)
                  (CallFunction|AjustSplineStartPositionandEndPosition (Variables|Default|GetSP_MultiplayerToMainMenu) (Variables|Default|2-Multiplayer|2.1-MultplayerToMainMenu|Get2%20-%20_MultiplayerPosition) (Variables|Default|2-Multiplayer|2.1-MultplayerToMainMenu|Get2%20-%20_MainMenuPosition) "Local"))
                (Variables|Default|2-Multiplayer|2.1-MultplayerToMainMenu|Set2%20-%20_MultiplayerPosition _initial_position)
                (Variables|Default|2-Multiplayer|2.1-MultplayerToMainMenu|Set2%20-%20_MainMenuPosition _end_position)
                (else
                  ;[1 1 1] Multiplayer Online to select spaceship camera animation
                  (if (Variables|Default|2-Multiplayer|2.2-MultplayerToSelectSpaceship|Get2%20-%20MultplayerToSelectSpaceship)
                    (CallFunction|CameraAnimation (Variables|Default|GetSP_MultiplayerToSelectSpaceship) (Variables|Default|2-Multiplayer|2.2-MultplayerToSelectSpaceship|Get2%20-%20_MultiplayerDistance_))))))))))))

(fn CameraAnimation
  (params (Spline :type Spline%20Component%20Object%20Reference) (Alpha :type Float%20%28double-precision%29))
  (Transformation|SetRelativeTransform (Variables|Default|GetCamera) (Spline|GetTransformatDistanceAlongSpline Spline (Math|Float|Lerp (Spline|GetDistanceAlongSplineatSplinePoint Spline 0) (Spline|GetDistanceAlongSplineatSplinePoint Spline (- (Spline|GetNumberOfSplinePoints Spline) 1)) Alpha) "Local" false) false false))

(fn SplineStartPositionandEndPosition
  (params (Spline :type Spline%20Component%20Object%20Reference) (CoordinateSpace :type ESplineCoordinateSpace%20Enum :default "Local"))
  (return (Spline|GetTransformatSplinePoint Spline 0 CoordinateSpace false) (Spline|GetTransformatSplinePoint Spline (- (Spline|GetNumberOfSplinePoints Spline) 1) CoordinateSpace false)))

(fn AjustSplineStartPositionandEndPosition
  (params (Spline :type Spline%20Component%20Object%20Reference) (InitialPosition :type Transform) (EndPosition :type Transform) (CoordinateSpace :type ESplineCoordinateSpace%20Enum :default "Local"))
  (bind (_location _rotation) (Math|Transform|BreakTransform EndPosition))
  (bind (_location_2 _rotation_2) (Math|Transform|BreakTransform InitialPosition))
  (bind _returnvalue (Spline|GetNumberOfSplinePoints Spline))
  (bind _returnvalue_2 (- _returnvalue 1))
  (Spline|SetLocationatSplinePoint Spline 0 _location_2 CoordinateSpace true)
  (Spline|SetRotationatSplinePoint Spline 0 _rotation_2 CoordinateSpace true)
  (Spline|SetLocationatSplinePoint Spline _returnvalue_2 _location CoordinateSpace true)
  (Spline|SetRotationatSplinePoint Spline _returnvalue_2 _rotation CoordinateSpace true)
  (return))